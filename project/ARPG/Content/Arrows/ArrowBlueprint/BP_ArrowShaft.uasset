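; BP_ArrowShaft is an arrow shaft Blueprint assembled from configurable static mesh components.
; Its construction script assigns meshes from variables to three components and sets a "texture" scalar material parameter on one of them, StaticMesh4, before swapping that component's mesh.
; The event graph holds only disabled placeholder events, so it adds no runtime logic.
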(fn `UserConstructionScript`
  (bind _staticmesh4 (`self.StaticMesh4`))
  (`MeshComponent.SetScalarParameterValueOnMaterials` _staticmesh4 "texture" (`self.NewVar_0`))
  (`StaticMeshComponent.SetStaticMesh` _staticmesh4 (`self.NewVar_1`))
  (`StaticMeshComponent.SetStaticMesh` (`self.StaticMesh2`) (`self.NewVar_2`))
  (`StaticMeshComponent.SetStaticMesh` (`self.StaticMesh1`) (`self.NewVar_3`)))